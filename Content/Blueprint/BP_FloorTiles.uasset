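; Floor tile for an endless-runner level that adds the next tile through LevelOneGameMode when the character crosses EndTrigger, then destroys itself two seconds later.
; Construction builds left, middle and right spawn points, then adds one randomly chosen child actor, item or obstacle, at a random point.
; Side-wall hits launch the character sideways along its right vector by BumpForce.
; GetAttachTransform exposes the attach point; CreateFoliage is an empty stub.
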(event `self.EndTrigger.OnComponentBeginOverlap`
  (params (OverlappedComponent :type "PrimitiveComponent Object Reference") (OtherActor :type "Actor Object Reference") (OtherComp :type "PrimitiveComponent Object Reference") (OtherBodyIndex :type Integer) (bFromSweep :type Boolean) (SweepResult :type "HitResult Structure (by ref)"))
  (cast `/Game/Jesus/ThirdPersonCharacter` OtherActor)
  (bind _aslevel_one_game_mode (cast `/Game/ControllerAndGameMode/LevelOneGameMode` (`GameplayStatics.GetGameMode`)))
  (`/Game/ControllerAndGameMode/LevelOneGameMode.AddFloorTile` _aslevel_one_game_mode)
  (`KismetSystemLibrary.Delay` 2.0)
  (`self.K2_DestroyActor`))

(event `self.Wall_L.OnComponentHit`
  (params (HitComponent :type "PrimitiveComponent Object Reference") (OtherActor :type "Actor Object Reference") (OtherComp :type "PrimitiveComponent Object Reference") (NormalImpulse :type "Vector Structure") (Hit :type "HitResult Structure (by ref)"))
  (bind _asthird_person_character (cast `/Game/Jesus/ThirdPersonCharacter` OtherActor))
  (`Character.LaunchCharacter` _asthird_person_character (* (`self.GetActorRightVector` _asthird_person_character) (`self.BumpForce`)) true false))

(event `self.Wall_R.OnComponentHit`
  (params (HitComponent :type "PrimitiveComponent Object Reference") (OtherActor :type "Actor Object Reference") (OtherComp :type "PrimitiveComponent Object Reference") (NormalImpulse :type "Vector Structure") (Hit :type "HitResult Structure (by ref)"))
  (bind _asthird_person_character (cast `/Game/Jesus/ThirdPersonCharacter` OtherActor))
  (`Character.LaunchCharacter` _asthird_person_character (* (* (`self.GetActorRightVector` _asthird_person_character) (`self.BumpForce`)) -1.0) true false))

(fn `CreateFoliage`)

(fn `GetAttachTransform`
  (returns (AttachTransform :type "Transform Structure"))
  (return (`SceneComponent.K2_GetComponentToWorld` (`self.AttachPoint`))))

(fn `SetSpawnPoints`
  (set `self.SpawnPoints` (`|MakeArray` (`SceneComponent.GetRelativeTransform` (`self.Left`)) (`SceneComponent.GetRelativeTransform` (`self.Middle`)) (`SceneComponent.GetRelativeTransform` (`self.Right`)))))

(fn `SpawnItems/Obstacle`
  (bind _output (`|GetArrayItem` (`self.SpawnPoints`) (`KismetMathLibrary.RandomIntegerInRange` 0 (`KismetArrayLibrary.Array_LastIndex` (`self.SpawnPoints`)))))
  (switch `int` (`KismetMathLibrary.RandomIntegerInRange` 0 3)
    (:`0`
      (`AddComponent|NODE_AddChildActorComponent-0` :`RelativeTransform` _output))
    (:`1`
      (`AddComponent|NODE_AddChildActorComponent-2` :`RelativeTransform` _output))
    (:`2`
      (`AddComponent|NODE_AddChildActorComponent-3` :`RelativeTransform` _output))
    (:`3`
      (`AddComponent|NODE_AddChildActorComponent-7` :`RelativeTransform` _output))))

(fn `UserConstructionScript`
  (`self.SetSpawnPoints`)
  (`self.SpawnItems/Obstacle`))